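; Game mode for the shooting game that provides functions to persist and retrieve the high score.
; SaveGameBP copies HighScore into a new ShootingSaveGame object and writes it to a configurable slot and user index.
; LoadGameBP returns the saved value from that slot, or zero when no save exists.
; The event graph runs no logic, holding only an unconnected SaveGameBP call.
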(fn `LoadGameBP`
  (returns (NewParam :type Integer))
  (bind _returnvalue (`GameplayStatics.DoesSaveGameExist` (`self.MySlotName`) (`self.MyUserIndex`)))
  (if _returnvalue
    (bind _returnvalue_2 (`GameplayStatics.LoadGameFromSlot` (`self.MySlotName`) (`self.MyUserIndex`)))
    (bind _asshooting_save_game (cast `ShootingSaveGame` _returnvalue_2))
    (return (`ShootingSaveGame.HighScoreSave` _asshooting_save_game))
    (else
      (return 0))))

(fn `SaveGameBP`
  (bind _returnvalue (`GameplayStatics.CreateSaveGameObject` "/Script/ShooingCpp.ShootingSaveGame"))
  (set `ShootingSaveGame.HighScoreSave` (`self.HighScore`) _returnvalue)
  (`GameplayStatics.SaveGameToSlot` _returnvalue (`self.MySlotName`) (`self.MyUserIndex`)))

(fn `UserConstructionScript`)